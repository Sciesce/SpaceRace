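; Snow ground actor that records rotated dig imprints into a render target read by its landscape material.
; Construction creates dynamic materials for the mesh and the dig brush, passing strength and up-multiplier settings to the brush.
; BeginPlay creates a white-cleared 8K render target and feeds it to the ground material's "Dis" parameter.
; GroundHit draws the brush into that target at the given UV and rotation, sized by DigScale, so imprints accumulate.
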(event Custom|GroundHit
  (params (UVLocation :type Vector%202D%20Structure) (Rotation :type Float%20%28single-precision%29))
  (bind (_canvas _size _context) (Rendering|BeginDrawCanvastoRenderTarget (Variables|Default|GetLand)))
  (Canvas|DrawMaterial :self _canvas :RenderMaterial (Variables|Default|GetImpact) :ScreenPosition (.Screen%20Position (CallFunction|SetCanvasMaterialScaleandPosition _size UVLocation (Variables|Default|GetDigScale))) :ScreenSize (.Screen%20Size (CallFunction|SetCanvasMaterialScaleandPosition _size UVLocation (Variables|Default|GetDigScale))) :Rotation (+ (* Rotation -1.0) -9e+01))
  (Rendering|EndDrawCanvastoRenderTarget _context))

(event EventBeginPlay
  (CallFunction|RenderTarget))

(fn ConstructionScript
  (bind _returnvalue (Rendering|Material|CreateDynamicMaterialInstance (Variables|Debug|GetStaticMeshComponent) 0 "/Game/Terrain/LandscapeSnow_Mat.LandscapeSnow_Mat" :!class /Script/Engine.PrimitiveComponent))
  (Variables|Default|SetGround _returnvalue)
  (bind _returnvalue_2 (Rendering|Material|CreateDynamicMaterialInstance "/Game/Terrain/Dig_Mat.Dig_Mat" :!class /Script/Engine.KismetMaterialLibrary))
  (Variables|Default|SetImpact _returnvalue_2)
  (Rendering|Material|SetScalarParameterValue (Variables|Default|GetImpact) "Strength" (Variables|Default|GetDigStrength) :!class /Script/Engine.MaterialInstanceDynamic)
  (Rendering|Material|SetScalarParameterValue (Variables|Default|GetImpact) "UpMulti" (Variables|Default|GetUpMulti) :!class /Script/Engine.MaterialInstanceDynamic))

(fn RenderTarget
  (bind _returnvalue (Rendering|CreateRenderTarget2D 8192 8192 "RTF_RGBA8"))
  (bind _output_get (Variables|Default|SetLand _returnvalue))
  (Rendering|ClearRenderTarget2D _output_get "(R=1.000000,G=1.000000,B=1.000000,A=1.000000)")
  (Rendering|Material|SetTextureParameterValue (Variables|Default|GetGround) "Dis" _output_get))