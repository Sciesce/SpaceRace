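; Wall Blueprint that continually cycles its static mesh through random colors.
; On BeginPlay it creates a dynamic material instance from Dynamic_example and starts a looping timer of about five seconds that calls ColorChange.
; Each ColorChange stores the previous color, picks a new random RGB, then plays a timeline that lerps between them into the ColorExample vector parameter for a gradual blend.
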(event Custom|ColorChange
  (Variables|Default|SetLinear%20Color%202 (Variables|Default|GetLinear%20Color%201))
  (Variables|Default|SetLinear%20Color%201 (Utilities|Struct|MakeLinearColor (Math|Random|RandomFloatinRange 0.0 1.0) (Math|Random|RandomFloatinRange 0.0 1.0) (Math|Random|RandomFloatinRange 0.0 1.0) 1.0))
  (bind _newtrack_0 (Timeline|Timeline_0 PlayFromStart)
    (:Update
      (Rendering|Material|SetVectorParameterValue (Variables|Default|GetDMI) "ColorExample" (Math|Color|Lerp(LinearColor) (Variables|Default|GetLinear%20Color%202) (Variables|Default|GetLinear%20Color%201) _newtrack_0) :!class /Script/Engine.MaterialInstanceDynamic))))

(event EventBeginPlay
  (bind _returnvalue (Rendering|Material|CreateDynamicMaterialInstance (Variables|Debug|GetStaticMeshComponent) 0 "/Game/Dynamic_Test/Dynamic_example.Dynamic_example" :!class /Script/Engine.PrimitiveComponent))
  (Variables|Default|SetDMI _returnvalue)
  (Utilities|Time|SetTimerbyFunctionName 0 "ColorChange" 5.001 true))

(fn ConstructionScript)